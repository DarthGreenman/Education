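; BP_RulesGame is a game rules Blueprint that handles the end conditions of a match: time running out or hero death.
; Two one-second looping timers count down GameDuration and poll BP_Hero's health.
; At zero time, QuitGame swaps all widgets for WBP_End and switches to UI-only input with a cursor.
; On death, a three-second QuitGame timer is set but cleared immediately, so it never fires.
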(event `self.ReceiveTick`
  (params (DeltaSeconds :type "Float (single-precision)")))

(event `self.ReceiveBeginPlay`
  (`self.ExecTimer`))

(fn `ConditionForDuration`
  (bind _result (`/Engine/EditorBlueprintResources/StandardMacros.DecrementInt` (`self.GameDuration`))
    (:`  `
      (if (== _result 0)
        (`KismetSystemLibrary.K2_ClearAndInvalidateTimerHandle` (`self.TimerHandlerDuration`))
        (`self.QuitGame`)))))

(fn `ConditionForHealth`
  (bind _returnvalue (`GameplayStatics.GetActorOfClass` "/Game/LeaveMeAlone/Core/Characters/BP_Hero.BP_Hero_C"))
  (if (<= (`Health.GetHealth` (`Hero.Health` _returnvalue)) 0.0)
    (`KismetSystemLibrary.K2_ClearAndInvalidateTimerHandle` (`self.TimerHandlerHealth`))
    (bind _returnvalue_2 (`KismetSystemLibrary.K2_SetTimer` null "QuitGame" 3.0 true))
    (`KismetSystemLibrary.K2_ClearAndInvalidateTimerHandle` _returnvalue_2)))

(fn `ExecTimer`
  (bind _returnvalue (`KismetSystemLibrary.K2_SetTimer` null "ConditionForDuration" 1.0 true))
  (set `self.TimerHandlerDuration` _returnvalue)
  (bind _returnvalue_2 (`KismetSystemLibrary.K2_SetTimer` null "ConditionForHealth" 1.0 true))
  (set `self.TimerHandlerHealth` _returnvalue_2))

(fn `QuitGame`
  (locals (NewLocalVar :type "SubmixEffectDelaySettings Structure"))
  (bind _returnvalue (`GameplayStatics.GetPlayerController` 0))
  (`WidgetLayoutLibrary.RemoveAllWidgets`)
  (bind _returnvalue_2 (`|CreateWidget` "/Game/LeaveMeAlone/Widgets/UI/WBP_End.WBP_End_C"))
  (`UserWidget.AddToViewport` _returnvalue_2 0)
  (`/Engine/EditorBlueprintResources/StandardMacros.IsValid` _returnvalue
    (:`Is Valid`
      (`WidgetBlueprintLibrary.SetInputMode_UIOnlyEx` _returnvalue null)
      (set `PlayerController.bShowMouseCursor` true _returnvalue))))

(fn `UserConstructionScript`)