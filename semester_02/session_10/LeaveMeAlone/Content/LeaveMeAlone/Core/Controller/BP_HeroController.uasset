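; Hero player controller Blueprint that opens the pause menu on the Pause input action.
; The press flips the OnPause flag through PerformPauseAction, which pauses the game, creates a new WBP_Pause widget, switches to UI-only input focused on it and shows the cursor.
; PerformPauseAction only stores its argument, so both toggle directions pause and add a widget; this graph has no resume path.
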(event `InputAction|Pause`
  (params (Key :type "Key Structure"))
  (:`Pressed`
    (if (`self.OnPause`)
      (`self.PerformPauseAction` false)
      (else
        (`self.PerformPauseAction` true)))))

(fn `PerformPauseAction`
  (params (OnPause :type Boolean))
  (bind _returnvalue (`GameplayStatics.GetPlayerController` 0))
  (set `self.OnPause` OnPause)
  (`GameplayStatics.SetGamePaused` true)
  (bind _returnvalue_2 (`|CreateWidget` "/Game/LeaveMeAlone/Widgets/UI/WBP_Pause.WBP_Pause_C"))
  (bind _output_get (set `self.PauseWidget` _returnvalue_2))
  (`UserWidget.AddToViewport` _output_get 0)
  (`/Engine/EditorBlueprintResources/StandardMacros.IsValid` _returnvalue
    (:`Is Valid`
      (`WidgetBlueprintLibrary.SetInputMode_UIOnlyEx` _returnvalue _returnvalue_2)
      (set `self.bShowMouseCursor` true))))

(fn `UserConstructionScript`)