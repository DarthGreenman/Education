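; BP_Selection is an invitation scene selection actor with a frame and a configurable inscription mesh that light up.
; The construction script adds the inscription component, zeroes both meshes' Brightness parameter and sets the actor unlocked.
; Overlapping it while unlocked calls the Unlock and ActivateSceneItem dispatchers.
; Activate tints the inscription and fades both meshes' brightness in through a timeline, while Deactivate locks the actor and reverses the fade.
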(event `self.ReceiveBeginPlay`)

(event `self.ReceiveActorBeginOverlap`
  (params (OtherActor :type "Actor Object Reference"))
  (if (`self.Un Locked`)
    (`self.Unlock`)
    (`self.Activate Scene Item`)))

(event `/Game/LeaveMeAlone/Interface/BPI_SceneItems.Activate`
  (params (Color :type "LinearColor Structure (by ref)"))
  (`/Game/LeaveMeAlone/Helper/BFL_HelperLibrary.Set Material Parameters for Component` Color (`self.Inscription Defined Later`))
  (bind (_direction _brightness) (`Timeline|Frame brightness Turn On-Off` :!label _label)
    (:`Update`
      (`MeshComponent.SetScalarParameterValueOnMaterials` (`self.Frame`) "Brightness" (`KismetMathLibrary.Lerp` 0.0 (`self.Brightness`) _brightness))
      (`MeshComponent.SetScalarParameterValueOnMaterials` (`self.Inscription Defined Later`) "Brightness" (`KismetMathLibrary.Lerp` 0.0 (`self.Brightness`) _brightness)))))

(event `/Game/LeaveMeAlone/Interface/BPI_SceneItems.Deactivate`
  (set `self.Un Locked` false)
  (goto _label :!via `Reverse`))

(fn `UserConstructionScript`
  (bind _returnvalue (`AddComponent|NODE_AddStaticMeshComponent-0`))
  (`StaticMeshComponent.SetStaticMesh` _returnvalue (`self.Inscription`))
  (bind _output_get (set `self.Inscription Defined Later` _returnvalue))
  (`MeshComponent.SetScalarParameterValueOnMaterials` _output_get "Brightness" 0.0)
  (`MeshComponent.SetScalarParameterValueOnMaterials` (`self.Frame`) "Brightness" 0.0)
  (set `self.Un Locked` true))