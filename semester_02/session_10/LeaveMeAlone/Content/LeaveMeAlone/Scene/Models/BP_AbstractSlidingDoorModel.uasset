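; Abstract sliding door model that opens and closes two leaves, judging by its name a base for door variants.
; The construction script stores each leaf's component, initial relative location and movement vector in a struct, negating the vector for the right leaf.
; Open plays a timeline that lerps each leaf's relative location from that start to the vector itself, used as an absolute target.
; Close reverses the timeline.
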(event `self.ReceiveBeginPlay`)

(event `self.Open`
  (bind (_leaf _position _moving) (break `/Game/LeaveMeAlone/Structures/F_SlidingDoorLeaf` (`self.Leaf Left Parametres`)))
  (bind (_leaf_2 _position_2 _moving_2) (break `/Game/LeaveMeAlone/Structures/F_SlidingDoorLeaf` (`self.Leaf Right Parametres`)))
  ; Кинематика
  (bind (_direction _moving_3) (`Timeline|Open And Close` :!label _label)
    (:`Update`
      (`SceneComponent.K2_SetRelativeLocation` _leaf_2 (`KismetMathLibrary.VLerp` _position_2 (`KismetMathLibrary.MakeVector` 0.0 _moving_2) _moving_3) false false)
      (`SceneComponent.K2_SetRelativeLocation` _leaf (`KismetMathLibrary.VLerp` _position (`KismetMathLibrary.MakeVector` 0.0 _moving) _moving_3) false false))))

(event `self.Close`
  ; Кинематика
  (goto _label :!via `Reverse`))

(fn `Get Door Leaf Motion Parameters`
  (params (Leaf :type "StaticMeshComponent Object Reference (by ref)") (Moving :type "Float (double-precision)"))
  (returns (`Returned Value` :type "/Game/LeaveMeAlone/Structures/F_SlidingDoorLeaf Structure"))
  (`/Engine/EditorBlueprintResources/StandardMacros.IsValid` Leaf
    (:`Is Valid`
      (return (make `/Game/LeaveMeAlone/Structures/F_SlidingDoorLeaf` Leaf (`SceneComponent.RelativeLocation` Leaf) Moving)))
    (:`Is Not Valid`
      (`KismetSystemLibrary.PrintString` "Leaf Is Not Valid"))))

(fn `UserConstructionScript`
  (bind _moving_the_door_leaf (`self.Moving the Door Leaf`))
  (set `self.Leaf Left Parametres` (`self.Get Door Leaf Motion Parameters` (`self.Leaf Left`) _moving_the_door_leaf))
  (set `self.Leaf Right Parametres` (`self.Get Door Leaf Motion Parameters` (`self.Leaf Right`) (* _moving_the_door_leaf -1.0))))