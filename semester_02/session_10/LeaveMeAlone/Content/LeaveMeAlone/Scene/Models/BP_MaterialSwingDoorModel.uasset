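; Swing door model that adds glowing, colorable columns, ornament and emblem to its parent's open and close behavior.
; The construction script creates ornament and emblem mesh components from configurable meshes, groups them with the columns and zeroes their Brightness parameter.
; Activate applies the given color to all three.
; Open plays a timeline that raises their material brightness to the configured level, and Close reverses it to fade the glow out.
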(event `/Game/LeaveMeAlone/Interface/BPI_SceneItems.Activate`
  (params (Color :type "LinearColor Structure (by ref)"))
  (for _array_element (`self.Components with Dynamic Material`)
    (`/Game/LeaveMeAlone/Helper/BFL_HelperLibrary.Set Material Parameters for Component` Color _array_element)))

(event `/Game/LeaveMeAlone/Interface/BPI_SceneItems.Deactivate`)

(event `/Game/LeaveMeAlone/Interface/BPI_Door.Open`
  (`parent.Open`)
  (bind (_direction _brightness) (`Timeline|Turn On And Off Entities with Dynamic Materials` :!label _label)
    (:`Update`
      (`MeshComponent.SetScalarParameterValueOnMaterials` (`self.Emblem Defined Later`) "Brightness" (`KismetMathLibrary.Lerp` 0.0 (`self.Brightness`) _brightness))
      (`MeshComponent.SetScalarParameterValueOnMaterials` (`self.Colums`) "Brightness" (`KismetMathLibrary.Lerp` 0.0 (`self.Brightness`) _brightness))
      (`MeshComponent.SetScalarParameterValueOnMaterials` (`self.Ornament Defined Later`) "Brightness" (`KismetMathLibrary.Lerp` 0.0 (`self.Brightness`) _brightness)))))

(event `/Game/LeaveMeAlone/Interface/BPI_Door.Close`
  (`parent.Close`)
  (goto _label :!via `Reverse`))

(fn `UserConstructionScript`
  (`parent.UserConstructionScript`)
  (`|ExecutionSequence`
    (:`then_0`
      (bind _returnvalue (`AddComponent|NODE_AddStaticMeshComponent-6`))
      (`StaticMeshComponent.SetStaticMesh` _returnvalue (`self.Ornament`))
      (set `self.Ornament Defined Later` _returnvalue))
    (:`then_1`
      (bind _returnvalue_2 (`AddComponent|NODE_AddStaticMeshComponent-7`))
      (`StaticMeshComponent.SetStaticMesh` _returnvalue_2 (`self.Emblem`))
      (set `self.Emblem Defined Later` _returnvalue_2))
    (:`then_2`
      (bind _output_get (set `self.Components with Dynamic Material` (`|MakeArray` (`self.Colums`) (`self.Ornament Defined Later`) (`self.Emblem Defined Later`))))
      (for _array_element _output_get
        (`MeshComponent.SetScalarParameterValueOnMaterials` _array_element "Brightness" 0.0)))))