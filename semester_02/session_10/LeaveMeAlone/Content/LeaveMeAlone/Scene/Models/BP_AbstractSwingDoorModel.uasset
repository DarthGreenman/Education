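; Abstract base model for a two-leaf swing door that animates both leaves open and closed.
; The construction script stores each leaf's component, initial relative rotation and opening angle in a swinging-leaf struct, negating the angle for the left leaf.
; Open plays a timeline that lerps each leaf from its stored rotation to that yaw, and Close reverses the same timeline.
; An invalid leaf prints a warning.
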(event `self.ReceiveBeginPlay`)

(event `self.Open`
  (bind (_leaf _position _angleofrotation) (break `/Game/LeaveMeAlone/Structures/F_SwingingDoorLeaf` (`self.Leaf Right Parametres`)))
  (bind (_leaf_2 _position_2 _angleofrotation_2) (break `/Game/LeaveMeAlone/Structures/F_SwingingDoorLeaf` (`self.Leaf Left Parametres`)))
  ; Кинематика
  (bind (_direction _rotation) (`Timeline|Open And Close` :!label _label)
    (:`Update`
      (`SceneComponent.K2_SetRelativeRotation` _leaf (`KismetMathLibrary.RLerp` _position (`KismetMathLibrary.MakeRotator` 0.0 0.0 _angleofrotation) _rotation) false false)
      (`SceneComponent.K2_SetRelativeRotation` _leaf_2 (`KismetMathLibrary.RLerp` _position_2 (`KismetMathLibrary.MakeRotator` 0.0 0.0 _angleofrotation_2) _rotation) false false))))

(event `self.Close`
  ; Кинематика
  (goto _label :!via `Reverse`))

(fn `Get Door Leaf Motion Parameters`
  (params (Leaf :type "StaticMeshComponent Object Reference (by ref)") (`Angel Of Rotation` :type "Float (double-precision)"))
  (returns (`Returned Value` :type "/Game/LeaveMeAlone/Structures/F_SwingingDoorLeaf Structure"))
  (`/Engine/EditorBlueprintResources/StandardMacros.IsValid` Leaf
    (:`Is Valid`
      (return (make `/Game/LeaveMeAlone/Structures/F_SwingingDoorLeaf` Leaf (`SceneComponent.RelativeRotation` Leaf) `Angel Of Rotation`)))
    (:`Is Not Valid`
      (`KismetSystemLibrary.PrintString` "Leaf Is Not Valid"))))

(fn `UserConstructionScript`
  (bind _angel_of_rotation (`self.Angel Of Rotation`))
  (set `self.Leaf Left Parametres` (`self.Get Door Leaf Motion Parameters` (`self.Leaf Left`) (* _angel_of_rotation -1.0)))
  (set `self.Leaf Right Parametres` (`self.Get Door Leaf Motion Parameters` (`self.Leaf Right`) _angel_of_rotation)))