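; Blueprint for an abstract model floor that lights up in a given color on Activate and dims again on Deactivate.
; Its construction script zeroes brightness on five regions and registers regions A, C and E as the dynamic-material components.
; Activate colors those three regions, then plays a timeline that lerps their Brightness parameter up to the configured value.
; Deactivate reverses the same timeline, while regions B and D stay dark.
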(event `self.ReceiveBeginPlay`)

(event `/Game/LeaveMeAlone/Interface/BPI_SceneItems.Activate`
  (params (Color :type "LinearColor Structure (by ref)"))
  (`|ExecutionSequence`
    (:`then_0`
      (for _array_element (`self.Components with Dynamic Material`)
        (`/Game/LeaveMeAlone/Helper/BFL_HelperLibrary.Set Material Parameters for Component` Color _array_element)))
    (:`then_1`
      (bind (_direction _brightness) (`Timeline|Turn on Turn off` :!label _label)
        (:`Update`
          (`MeshComponent.SetScalarParameterValueOnMaterials` (`self.Region A`) "Brightness" (`KismetMathLibrary.Lerp` 0.0 (`self.Brightness`) _brightness))
          (`MeshComponent.SetScalarParameterValueOnMaterials` (`self.Region C`) "Brightness" (`KismetMathLibrary.Lerp` 0.0 (`self.Brightness`) _brightness))
          (`MeshComponent.SetScalarParameterValueOnMaterials` (`self.Region E`) "Brightness" (`KismetMathLibrary.Lerp` 0.0 (`self.Brightness`) _brightness)))))))

(event `self.Deactivate`
  (goto _label :!via `Reverse`))

(fn `UserConstructionScript`
  (`MeshComponent.SetScalarParameterValueOnMaterials` (`self.Region A`) "Brightness" 0.0)
  (`MeshComponent.SetScalarParameterValueOnMaterials` (`self.Region B`) "Brightness" 0.0)
  (`MeshComponent.SetScalarParameterValueOnMaterials` (`self.Region C`) "Brightness" 0.0)
  (`MeshComponent.SetScalarParameterValueOnMaterials` (`self.Region D`) "Brightness" 0.0)
  (`MeshComponent.SetScalarParameterValueOnMaterials` (`self.Region E`) "Brightness" 0.0)
  (set `self.Components with Dynamic Material` (`|MakeArray` (`self.Region A`) (`self.Region C`) (`self.Region E`))))