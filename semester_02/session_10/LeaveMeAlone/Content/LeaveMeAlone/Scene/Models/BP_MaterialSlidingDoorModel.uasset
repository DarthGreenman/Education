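; Sliding door model Blueprint that lights up its frame material as the door opens and dims it as it closes.
; Activate applies the given color to the Frame's material parameters, while Deactivate is empty.
; Open and Close call the parent behavior, then play or reverse a timeline that lerps the Frame's Brightness scalar between its min and max.
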(event `/Game/LeaveMeAlone/Interface/BPI_SceneItems.Activate`
  (params (Color :type "LinearColor Structure (by ref)"))
  (`/Game/LeaveMeAlone/Helper/BFL_HelperLibrary.Set Material Parameters for Component` Color (`self.Frame`)))

(event `/Game/LeaveMeAlone/Interface/BPI_SceneItems.Deactivate`)

(event `/Game/LeaveMeAlone/Interface/BPI_Door.Open`
  (bind (_min _max) (break `FloatInterval` (`self.Brightness`)))
  (`parent.Open`)
  (bind (_direction _brightness) (`Timeline|Turn On And Off Entities with Dynamic Materials` :!label _label)
    (:`Update`
      (`MeshComponent.SetScalarParameterValueOnMaterials` (`self.Frame`) "Brightness" (`KismetMathLibrary.Lerp` _min _max _brightness)))))

(event `/Game/LeaveMeAlone/Interface/BPI_Door.Close`
  (`parent.Close`)
  (goto _label :!via `Reverse`))

(fn `UserConstructionScript`
  (`parent.UserConstructionScript`))