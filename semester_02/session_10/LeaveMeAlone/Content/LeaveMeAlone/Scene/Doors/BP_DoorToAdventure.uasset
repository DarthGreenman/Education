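; Door Blueprint for the adventure entrance, layering sounds and scene-item deactivation onto inherited door behavior.
; Opening clears UnLocked, plays the opening sound and fires the DeactivateSceneItem dispatcher for two enum item types.
; Leaving the capsule collision calls Close, which plays a stone sound only while UnLocked is false.
; The construction script starts UnLocked as true, so that sound is skipped until Open has run.
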(event `self.ReceiveBeginPlay`
  (`parent.ReceiveBeginPlay`))

(event `/Game/LeaveMeAlone/Interface/BPI_Door.Open`
  (`parent.Open`)
  (set `self.Un Locked` false)
  (`|ExecutionSequence`
    (:`then_0`
      (`GameplayStatics.PlaySound2D` "/Game/LeaveMeAlone/Ambient/S_OpenDoor.S_OpenDoor" (`self.Volume Multiplier Door Opening`) 1.0 0.0 null null))
    (:`then_1`
      (`self.Deactivate Scene Item` "NewEnumerator1")
      (`self.Deactivate Scene Item` "NewEnumerator0"))))

(event `/Game/LeaveMeAlone/Interface/BPI_Door.Close`
  (`parent.Close`)
  (if (not (`self.Un Locked`))
    (`GameplayStatics.PlaySound2D` "/Game/LeaveMeAlone/Sound/StoneDoor.StoneDoor" (`self.Volume Multiplier Door Opening`) 1.0 0.0 null null)))

(event `/Game/LeaveMeAlone/Interface/BPI_SceneItems.Activate`
  (params (Color :type "LinearColor Structure (by ref)"))
  (`parent.Activate` Color))

(event `/Game/LeaveMeAlone/Interface/BPI_SceneItems.Deactivate`
  (`parent.Deactivate`))

(event `self.Capsule Collision.OnComponentEndOverlap`
  (params (OverlappedComponent :type "PrimitiveComponent Object Reference") (OtherActor :type "Actor Object Reference") (OtherComp :type "PrimitiveComponent Object Reference") (OtherBodyIndex :type Integer))
  (`/Game/LeaveMeAlone/Interface/BPI_Door.Close`))

(fn `UserConstructionScript`
  (`parent.UserConstructionScript`)
  (set `self.Un Locked` true))