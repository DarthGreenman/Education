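; Teleport floor tile that, when overlapped, moves the overlapping actor to an offset from the level's BP_Hexagon.
; Overlap starts two parallel delayed chains: one plays a countdown sound, then spins RegionB and RegionC through a timeline.
; The other waits the construction-set period, teleports the actor, broadcasts ActivateSceneItem with the color stored on Activate, and plays the teleport sound.
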(event `/Game/LeaveMeAlone/Interface/BPI_SceneItems.Activate`
  (params (Color :type "LinearColor Structure (by ref)"))
  (bind _output_get (set `self.Color` Color))
  (`parent.Activate` _output_get))

(event `/Game/LeaveMeAlone/Interface/BPI_SceneItems.Deactivate`
  (`parent.Deactivate`))

(event `self.Teleport.OnComponentBeginOverlap`
  (params (OverlappedComponent :type "PrimitiveComponent Object Reference") (OtherActor :type "Actor Object Reference") (OtherComp :type "PrimitiveComponent Object Reference") (OtherBodyIndex :type Integer) (bFromSweep :type Boolean) (SweepResult :type "HitResult Structure (by ref)"))
  (`|ExecutionSequence`
    (:`then_0`
      (`KismetSystemLibrary.Delay` 1.0)
      (`GameplayStatics.PlaySound2D` "/Game/LeaveMeAlone/Sound/Countdown.Countdown" 2.0 1.0 0.0 null null)
      (`KismetSystemLibrary.Delay` 2.0)
      (bind (_direction _rotation) (`Timeline|Launching the Teleport`)
        (:`Update`
          (`SceneComponent.K2_AddRelativeRotation` (`self.Region B`) (`KismetMathLibrary.MakeRotator` 0.0 0.0 (`KismetMathLibrary.Lerp` 0.0 180.0 _rotation)) false false)
          (`SceneComponent.K2_AddRelativeRotation` (`self.Region C`) (`KismetMathLibrary.MakeRotator` 0.0 0.0 (`KismetMathLibrary.Lerp` 0.0 180.0 _rotation)) false false))))
    (:`then_1`
      (`KismetSystemLibrary.Delay` (`self.Time Period before Teleportation`))
      (bind _returnvalue (`GameplayStatics.GetActorOfClass` "/Game/LeaveMeAlone/Scene/BP_Hexagon.BP_Hexagon_C"))
      (`self.K2_SetActorLocation` OtherActor (+ (`self.K2_GetActorLocation` _returnvalue) (`KismetMathLibrary.MakeVector` (* -3058.36478 0.75))) false true)
      (`self.Activate Scene Item` (`self.Color`))
      (`GameplayStatics.PlaySound2D` "/Game/LeaveMeAlone/Sound/Teleport.Teleport" 1.0 1.0 0.0 null null))))

(fn `UserConstructionScript`
  (`parent.UserConstructionScript`)
  (set `self.Time Period before Teleportation` 13.0))