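; BP_Hexagon is a scene actor that spawns enemies and lights up hexagon floor places with a color supplied by BP_Portal.
; It binds to the portal's activation event, stores the color and spawns BP_Enemy actors at random offsets and yaws around itself.
; While unlocked, overlapping ArrivalPlace plays a heartbeat sound and activates the inner and outer floor hexagons after a short delay.
; Leaving ArrivalPlace locks it against retriggering.
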(event `self.ReceiveBeginPlay`
  (bind _returnvalue (`GameplayStatics.GetActorOfClass` "/Game/LeaveMeAlone/Scene/BP_Portal.BP_Portal_C"))
  (add `/Game/LeaveMeAlone/Scene/BP_Portal.Activate Scene Item` _returnvalue (delegate `Activate Hexagon`)))

(event `Activate Hexagon`
  (params (Color :type "LinearColor Structure (by ref)") (`Number of Enemies` :type Integer))
  (set `self.Color` Color)
  (`self.Spawning the Enemies` `Number of Enemies`))

(event `self.ReceiveActorBeginOverlap`
  (params (OtherActor :type "Actor Object Reference")))

(event `self.Arrival Place.OnComponentBeginOverlap`
  (params (OverlappedComponent :type "PrimitiveComponent Object Reference") (OtherActor :type "Actor Object Reference") (OtherComp :type "PrimitiveComponent Object Reference") (OtherBodyIndex :type Integer) (bFromSweep :type Boolean) (SweepResult :type "HitResult Structure (by ref)"))
  (bind _color (`self.Color`))
  (if (`self.Un Locked`)
    (`KismetSystemLibrary.Delay` 1.0)
    (`|ExecutionSequence`
      (:`then_0`
        (`GameplayStatics.PlaySound2D` "/Game/LeaveMeAlone/Sound/BreathingWithHeartbeat.BreathingWithHeartbeat" 4.0 1.0 0.0 null null)
        (`KismetSystemLibrary.Delay` 5.0))
      (:`then_1`
        (bind _returnvalue (`GameplayStatics.GetActorOfClass` "/Game/LeaveMeAlone/Scene/Floors/BP_FloorPlaceHexagonInner.BP_FloorPlaceHexagonInner_C"))
        (`/Game/LeaveMeAlone/Interface/BPI_SceneItems.Activate` _returnvalue _color)
        (bind _returnvalue_2 (`GameplayStatics.GetActorOfClass` "/Game/LeaveMeAlone/Scene/Floors/BP_FloorPlaceHexagonOuter.BP_FloorPlaceHexagonOuter_C"))
        (`/Game/LeaveMeAlone/Interface/BPI_SceneItems.Activate` _returnvalue_2 _color)))))

(event `self.Arrival Place.OnComponentEndOverlap`
  (params (OverlappedComponent :type "PrimitiveComponent Object Reference") (OtherActor :type "Actor Object Reference") (OtherComp :type "PrimitiveComponent Object Reference") (OtherBodyIndex :type Integer))
  (set `self.Un Locked` false))

(fn `Make Random Transform`
  (params (Abscissa :type "FloatInterval Structure") (Ordinate :type "FloatInterval Structure"))
  (returns (Transform :type "Transform Structure"))
  (bind _returnvalue (`self.GetTransform`))
  (return (`KismetMathLibrary.MakeTransform` (`KismetMathLibrary.MakeVector` (+ (.x (.location _returnvalue)) (`KismetMathLibrary.RandomFloatInRange` Abscissa_Min Abscissa_Max)) (+ (`KismetMathLibrary.RandomFloatInRange` Ordinate_Min Ordinate_Max) (.y (.location _returnvalue)))) (`KismetMathLibrary.MakeRotator` 0.0 0.0 (+ (`KismetMathLibrary.RandomFloatInRange` 0.0 360.0) (.yaw (.rotation _returnvalue)))))))

(fn `Spawning the Enemies`
  (params (`Number Of Enemies` :type Integer))
  (for _ (range (+ `Number Of Enemies` 1))
    (`|SpawnActorFromClass` "/Game/LeaveMeAlone/Core/Characters/BP_Enemy.BP_Enemy_C" (`self.Make Random Transform` (make `FloatInterval` -1000.0 1000.0) (make `FloatInterval` -1000.0 1000.0)) "AdjustIfPossibleButAlwaysSpawn" "MultiplyWithRoot" null null))
  (return))

(fn `UserConstructionScript`
  (set `self.Un Locked` true))